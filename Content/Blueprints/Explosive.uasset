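; Explosive is a hazard built on a pickup parent class that damages and launches the player's BallPawn.
; On BeginPlay it sets explosion effects and no score points, plays a spark sound, and binds itself to the pawn's destroy-hazards event.
; Pickup applies a radial impulse from below the explosive and subtracts Damage from Health, clamped at zero.
; The destroy event spawns a sparkle, then explodes audibly and removes the actor after a short delay.
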(event `self.ReceiveBeginPlay`
  (set `self.UseNumberWidget` false)
  (set `self.Points` 0)
  (set `self.PickupSound` "/Game/StarterContent/Audio/Explosion01.Explosion01")
  (set `self.OnPickupParticles` "/Game/StarterContent/Particles/P_Explosion.P_Explosion")
  (`GameplayStatics.PlaySoundAtLocation` "/Game/StarterContent/Audio/Fire_Sparks01_Cue.Fire_Sparks01_Cue" (`self.K2_GetActorLocation`) (struct) 1.0 1.0 0.0 null null null)
  (`parent.ReceiveBeginPlay`)
  (add `/Game/Blueprints/BallPawn.DestroyHazards` (cast `/Game/Blueprints/BallPawn` (`GameplayStatics.GetPlayerPawn` 0) :!pure true) (delegate `DestroySelf`)))

(event `DestroySelf`
  (`GameplayStatics.SpawnEmitterAtLocation` "/Game/InfinityBladeEffects/Effects/FX_Treasure/Gold_Bag/P_GoldSparkle_Bag_Pickup.P_GoldSparkle_Bag_Pickup" (`self.K2_GetActorLocation`))
  (`KismetSystemLibrary.Delay` 0.75)
  (`GameplayStatics.PlaySound2D` "/Game/StarterContent/Audio/Explosion01.Explosion01" 1.0 1.0 0.0 null null)
  (`self.K2_DestroyActor`))

(event `self.OnPickup`
  (params (OtherActor :type "Object Object Reference"))
  (bind _asball_pawn (cast `/Game/Blueprints/BallPawn` OtherActor))
  (`PrimitiveComponent.AddRadialImpulse` (`/Game/Blueprints/BallPawn.BallMesh` _asball_pawn) (`KismetMathLibrary.MakeVector` (.x (`self.K2_GetActorLocation`)) (.y (`self.K2_GetActorLocation`)) (+ (.z (`self.K2_GetActorLocation`)) -75.0)) 500.0 500.0 "RIF_Constant" true)
  (bind _returnvalue (- (`/Game/Blueprints/BallPawn.Health` _asball_pawn) (`self.Damage`)))
  (if (< _returnvalue 0)
    (set `/Game/Blueprints/BallPawn.Health` 0 _asball_pawn)
    (else
      (set `/Game/Blueprints/BallPawn.Health` _returnvalue _asball_pawn)))
  (`parent.OnPickup` OtherActor))

(fn `UserConstructionScript`
  (`parent.UserConstructionScript`))