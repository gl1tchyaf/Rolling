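; Booster button that launches the player's BallPawn along the button's up vector when the ball hits it.
; A BallPawn entering the trigger box plays a sound and a timeline that offsets the button's Z from its initial location.
; Leaving the box reverses the timeline after a one-second delay.
; Hits on the button apply a velocity-change impulse to the ball mesh, ignoring its mass.
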(event `self.ReceiveBeginPlay`
  (set `self.InitialButtonLocation` (`SceneComponent.K2_GetComponentLocation` (`self.Button`))))

(event `self.Box.OnComponentBeginOverlap`
  (params (OverlappedComponent :type "PrimitiveComponent Object Reference") (OtherActor :type "Actor Object Reference") (OtherComp :type "PrimitiveComponent Object Reference") (OtherBodyIndex :type Integer) (bFromSweep :type Boolean) (SweepResult :type "HitResult Structure (by ref)"))
  (cast `/Game/Blueprints/BallPawn` OtherActor)
  (`GameplayStatics.PlaySound2D` "/Game/Retro_8Bit_Sounds/Collectables/Cues/retro_collect_pickup_item_08_Cue.retro_collect_pickup_item_08_Cue" 1.0 1.0 0.0 null null)
  (bind (_direction _buttonelevation2) (`Timeline|ButtonTimeline` :!label _label)
    (:`Update`
      (`self.Update Button` _buttonelevation2))))

(event `self.Box.OnComponentEndOverlap`
  (params (OverlappedComponent :type "PrimitiveComponent Object Reference") (OtherActor :type "Actor Object Reference") (OtherComp :type "PrimitiveComponent Object Reference") (OtherBodyIndex :type Integer))
  (cast `/Game/Blueprints/BallPawn` OtherActor)
  (`KismetSystemLibrary.Delay` 1.0)
  (goto _label :!via `Reverse`))

(event `self.Button.OnComponentHit`
  (params (HitComponent :type "PrimitiveComponent Object Reference") (OtherActor :type "Actor Object Reference") (OtherComp :type "PrimitiveComponent Object Reference") (NormalImpulse :type "Vector Structure") (Hit :type "HitResult Structure (by ref)"))
  (bind _asball_pawn (cast `/Game/Blueprints/BallPawn` OtherActor))
  (`PrimitiveComponent.AddImpulse` (`/Game/Blueprints/BallPawn.BallMesh` _asball_pawn) (* (`SceneComponent.GetUpVector` (`self.Button`)) (`self.Impulse`)) "None" true))

(fn `Update Button`
  (params (ButtonElevation :type "Float (double-precision)"))
  (`|ExecutionSequence`
    (:`then_0`
      (`SceneComponent.K2_SetWorldLocation` (`self.Button`) (`KismetMathLibrary.MakeVector` (.x (`self.InitialButtonLocation`)) (.y (`self.InitialButtonLocation`)) (+ (.z (`self.InitialButtonLocation`)) ButtonElevation)) false false))))

(fn `UserConstructionScript`)