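; A one-shot floor button that a BallPawn presses by overlapping its sphere, triggering the actors in AffectedActors.
; Pressing plays a sound, turns the dynamic material instance red and drives the mesh height through a timeline.
; It then calls OnPickup on each linked Button or LaunchActor.
; A Button's own OnPickup re-arms it by restoring orange and reversing the timeline, so buttons can reset one another.
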(event `self.ReceiveBeginPlay`
  ;[1 1 1] Begin Play
  (set `self.InitialButtonLocation` (`SceneComponent.K2_GetComponentLocation` (`self.Button`))))

(event `self.OverlapSphere.OnComponentBeginOverlap`
  (params (OverlappedComponent :type "PrimitiveComponent Object Reference") (OtherActor :type "Actor Object Reference") (OtherComp :type "PrimitiveComponent Object Reference") (OtherBodyIndex :type Integer) (bFromSweep :type Boolean) (SweepResult :type "HitResult Structure (by ref)"))
  (cast `/Game/Blueprints/BallPawn` OtherActor)
  ;[1 1 1] Check if button down
  (if (not (`self.ButtonDown`))
    (`GameplayStatics.PlaySound2D` "/Game/Retro_8Bit_Sounds/Collectables/Cues/retro_collect_pickup_item_08_Cue.retro_collect_pickup_item_08_Cue" 1.0 1.0 0.0 null null)
    (set `self.ButtonDown` true)
    ;[1 1 1] Set color to red
    (`MaterialInstanceDynamic.SetVectorParameterValue` (`self.OrangeMaterialInst`) "Color" (struct :`R` 1.0 :`B` 0.038562 :`A` 1.0))
    (for _array_element (`self.AffectedActors`)
      (bind _asbutton (cast `/Game/Blueprints/Button` _array_element)
        (:`then`
          (`/Game/Blueprints/ButtonInterface.OnPickup` _asbutton))
        (:`CastFailed`
          (bind _aslaunch_actor (cast `/Game/Blueprints/LaunchActor` _array_element))
          (`/Game/Blueprints/ButtonInterface.OnPickup` _aslaunch_actor))))
    (bind (_direction _buttonelevation) (`Timeline|ButtonTimeline` :!label _label)
      (:`Update`
        (`SceneComponent.K2_SetWorldLocation` (`self.Button`) (`KismetMathLibrary.MakeVector` (.x (`self.InitialButtonLocation`)) (.y (`self.InitialButtonLocation`)) (+ (.z (`self.InitialButtonLocation`)) _buttonelevation)) false false)))))

(event `/Game/Blueprints/ButtonInterface.OnPickup`
  (`MaterialInstanceDynamic.SetVectorParameterValue` (`self.OrangeMaterialInst`) "Color" (struct :`R` 0.8 :`G` 0.3 :`A` 1.0))
  (set `self.ButtonDown` false)
  (goto _label :!via `Reverse`))

(fn `UserConstructionScript`
  (bind _returnvalue (`KismetMaterialLibrary.CreateDynamicMaterialInstance` "/Game/Blueprints/Materials/ButtonMaterial.ButtonMaterial"))
  (bind _output_get (set `self.OrangeMaterialInst` _returnvalue))
  (`PrimitiveComponent.SetMaterial` (`self.Button`) 0 _output_get))